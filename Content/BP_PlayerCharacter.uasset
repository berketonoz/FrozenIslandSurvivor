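; Networked player character that switches movement gates on aim input and seeds its storage component with two starting items when locally controlled.
; Aim start and end send the gate through server-to-multicast RPCs to UpdateGate, which notifies the AnimInstance and applies that gate's CharacterMovement settings from a GateSettings map.
; Montage playback uses the same server-to-multicast relay, and debug keys set global time dilation through a server RPC.
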(event Custom|RPC_Multicast_UpdateGate
  (params (Gate :type E_Gate%20Enum :default "NewEnumerator0"))
  ;[0.15 0.15 0.15 0.5] Aim Action
  (CallFunction|UpdateGate Gate))

(event Custom|RPC_Server_UpdateGate
  (params (Gate :type E_Gate%20Enum :default "NewEnumerator0"))
  ;[0.15 0.15 0.15 0.5] Aim Action
  (CallFunction|RPCMulticastUpdateGate Gate))

(event Custom|RPC_Server_TimeDilation
  (params (TimeDilation :type Float%20%28double-precision%29))
  ;[0.15 0.15 0.15 0.5] Debug By Time Dilation
  (Utilities|Time|SetGlobalTimeDilation TimeDilation))

(event Custom|RPC_Server_AnimationMontage
  (params (AnimMontage :type Anim%20Montage%20Object%20Reference))
  (CallFunction|RPCMulticastAnimationMontage AnimMontage))

(event Custom|RPC_Multicast_AnimationMontage
  (params (AnimMontage :type Anim%20Montage%20Object%20Reference))
  (Animation|PlayAnimMontage AnimMontage 1.0 "None"))

(event Input|EnhancedActionEvents|EnhancedInputActionIA_Aim
  (params (ActionValue :type Boolean) (ElapsedSeconds :type Float%20%28double-precision%29) (TriggeredSeconds :type Float%20%28double-precision%29) (InputAction :type Input%20Action%20Object%20Reference :default "/Game/Inputs/Actions/IA_Aim.IA_Aim"))
  ;[0.15 0.15 0.15 0.5] Aim Action
  (:Started
    (CallFunction|RPCServerUpdateGate "NewEnumerator0"))
  (:Completed
    (CallFunction|RPCServerUpdateGate "NewEnumerator1")))

(event EventBeginPlay
  ;[0.05098 0.05098 0.05098] Event BeginPlay & Tick
  (if (Pawn|IsLocallyControlled)
    (Class|StorageComponent|ServerAddBPItem (Variables|Default|GetStorageComponent) (Utilities|Struct|MakeInventoryItem "03_snow" 2 1 false true 0) -1)
    (Class|StorageComponent|ServerAddBPItem (Variables|Default|GetStorageComponent) (Utilities|Struct|MakeInventoryItem "01_bread" 1 1 false true 0) -1)))

(event Input|KeyboardEvents|DebugKeySubtract
  (params (Key :type Key%20Structure :default "None") (ActionValue :type Input%20Action%20Value%20Structure))
  ;[0.15 0.15 0.15 0.5] Debug By Time Dilation
  (:Pressed
    (CallFunction|RPCServerTimeDilation 0.1)))

(event Input|KeyboardEvents|DebugKeyAdd
  (params (Key :type Key%20Structure :default "None") (ActionValue :type Input%20Action%20Value%20Structure))
  ;[0.15 0.15 0.15 0.5] Debug By Time Dilation
  (:Pressed
    (CallFunction|RPCServerTimeDilation 1.0)))

(fn ConstructionScript)

(fn UpdateGate
  (params (Gate :type E_Gate%20Enum :default "NewEnumerator0"))
  (bind _charactermovement (Variables|Character|GetCharacterMovement))
  (bind _output_get (Variables|Default|SetCurrentGate Gate))
  (Class|BPIAnimationInterface|RecieveCurrentGate(Message) (Components|SkeletalMesh|GetAnimInstance (Variables|Character|GetMesh)) _output_get)
  (Utilities|FlowControl|Sequence
    (:then_0
      (Variables|/Script/Engine.CharacterMovementComponent|SetMaxWalkSpeed _charactermovement (.MaxWalkSpeed (Utilities|Struct|BreakS_GateSetting (.Value (Utilities|Map|Find (Variables|Default|GetGateSettings) _output_get))))))
    (:then_1
      (Variables|/Script/Engine.CharacterMovementComponent|SetMaxAcceleration _charactermovement (.MaxAcceleration (Utilities|Struct|BreakS_GateSetting (.Value (Utilities|Map|Find (Variables|Default|GetGateSettings) _output_get))))))
    (:then_2
      (Variables|/Script/Engine.CharacterMovementComponent|SetBrakingDecelerationWalking _charactermovement (.BrakingDeceleration (Utilities|Struct|BreakS_GateSetting (.Value (Utilities|Map|Find (Variables|Default|GetGateSettings) _output_get))))))
    (:then_3
      (Variables|/Script/Engine.CharacterMovementComponent|SetBrakingFrictionFactor _charactermovement (.BrakingFrictionFactor (Utilities|Struct|BreakS_GateSetting (.Value (Utilities|Map|Find (Variables|Default|GetGateSettings) _output_get))))))
    (:then_4
      (Variables|/Script/Engine.CharacterMovementComponent|SetBrakingFriction _charactermovement (.BrakingFriction (Utilities|Struct|BreakS_GateSetting (.Value (Utilities|Map|Find (Variables|Default|GetGateSettings) _output_get))))))
    (:then_5
      (Variables|/Script/Engine.CharacterMovementComponent|SetbUseSeparateBrakingFriction _charactermovement (.UseSeparateBrakingFriction (Utilities|Struct|BreakS_GateSetting (.Value (Utilities|Map|Find (Variables|Default|GetGateSettings) _output_get))))))))