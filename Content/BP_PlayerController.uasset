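; Player controller that manages the player's HUD screens and a building rotation input.
; After a short delay on BeginPlay, the local controller adds a crosshair and pre-creates inventory storage, preview and build menu widgets.
; Tab, I and B toggle those screens independently, switching input mode and mouse cursor with each.
; R forwards a rotate call to the pawn's BuildComponent on BP_PlayerCharacter.
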(event `self.ReceiveBeginPlay`
  (`KismetSystemLibrary.Delay` 0.5)
  (if (`self.IsLocalController`)
    (bind _returnvalue (`|CreateWidget` "/Game/UI/CrossHairs/CrossHair.CrossHair_C" self (`self.CrossHairSize`)))
    (`UserWidget.AddToViewport` _returnvalue 0)
    (bind _returnvalue_2 (`|CreateWidget` "/Game/UI/HUDs/PlayerStorageHUD.PlayerStorageHUD_C" self))
    (set `self.PlayerStorageHUD` _returnvalue_2)
    (bind _returnvalue_3 (`|CreateWidget` "/Game/UI/HUDs/PreviewHUD.PreviewHUD_C" self))
    (set `self.PreviewHUD` _returnvalue_3)
    (bind _returnvalue_4 (`|CreateWidget` "/Game/UI/HUDs/BuildMenuHUD.BuildMenuHUD_C" self))
    (set `self.BuildMenuHUD` _returnvalue_4)))

(event `ShowInventory`
  (bind _playerstoragehud (`self.PlayerStorageHUD`))
  ; Show & Hide Inventory Storage
  (`WidgetBlueprintLibrary.SetInputMode_GameAndUIEx` self null)
  (`/Engine/EditorBlueprintResources/StandardMacros.IsValid` _playerstoragehud
    (:`Is Valid`
      (`UserWidget.AddToViewport` _playerstoragehud 0)
      (set `self.IsInventoryOpen` true)
      (set `self.bShowMouseCursor` true))))

(event `ShowPreview`
  (bind _previewhud (`self.PreviewHUD`))
  ; Show & Hide Preview Screen
  (`WidgetBlueprintLibrary.SetInputMode_GameAndUIEx` self null)
  (`/Engine/EditorBlueprintResources/StandardMacros.IsValid` _previewhud
    (:`Is Valid`
      (`UserWidget.AddToViewport` _previewhud 0)
      (set `self.IsPreviewOpen` true)
      (set `self.bShowMouseCursor` true))))

(event `HideInventory`
  ; Show & Hide Inventory Storage
  (`WidgetBlueprintLibrary.SetInputMode_GameOnly` self)
  (`Widget.RemoveFromParent` (`self.PlayerStorageHUD`))
  (set `self.IsInventoryOpen` false)
  (set `self.bShowMouseCursor` false))

(event `HidePreview`
  ; Show & Hide Preview Screen
  (`WidgetBlueprintLibrary.SetInputMode_GameOnly` self)
  (`Widget.RemoveFromParent` (`self.PreviewHUD`))
  (set `self.IsPreviewOpen` false)
  (set `self.bShowMouseCursor` false))

(event `Key|I`
  (params (Key :type "Key Structure"))
  ; Toggle Preview Screen
  (:`Pressed`
    (if (`self.IsPreviewOpen`)
      (`self.HidePreview`)
      (else
        (`self.ShowPreview`)))))

(event `Key|Tab`
  (params (Key :type "Key Structure"))
  ; Toggle Inventory
  (:`Pressed`
    (if (`self.IsInventoryOpen`)
      (`self.HideInventory`)
      (else
        (`self.ShowInventory`)))))

(event `ShowBuildMenu`
  (bind _buildmenuhud (`self.BuildMenuHUD`))
  ; Show & Hide Build Menu
  (`WidgetBlueprintLibrary.SetInputMode_GameAndUIEx` self null)
  (`/Engine/EditorBlueprintResources/StandardMacros.IsValid` _buildmenuhud
    (:`Is Valid`
      (`UserWidget.AddToViewport` _buildmenuhud 0)
      (set `self.IsBuildOpen` true)
      (set `self.bShowMouseCursor` true))))

(event `HideBuildMenu`
  ; Show & Hide Build Menu
  (`WidgetBlueprintLibrary.SetInputMode_GameOnly` self)
  (`Widget.RemoveFromParent` (`self.BuildMenuHUD`))
  (set `self.IsBuildOpen` false)
  (set `self.bShowMouseCursor` false))

(event `Key|B`
  (params (Key :type "Key Structure"))
  ; Toggle Build Menu
  (:`Pressed`
    (if (`self.IsBuildOpen`)
      (`self.HideBuildMenu`)
      (else
        (`self.ShowBuildMenu`)))))

(event `Key|R`
  (params (Key :type "Key Structure"))
  ; Rotate Building
  (:`Pressed`
    (bind _asbp_player_character (cast `/Game/BP_PlayerCharacter` (`self.K2_GetPawn`)))
    (`BuildComponent.RotateBuilding` (`FrozenIslandCharacter.BuildComponent` _asbp_player_character) 1.0)))

(fn `UserConstructionScript`)